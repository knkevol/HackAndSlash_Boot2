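; Game state Blueprint for the HackAndSlash mode, tracking the current game state and an accumulated time counter.
; Tick adds frame delta to TotalDeltaSeconds, which ChangeGameState resets on every call, even if the requested state is already active.
; When the state differs, ChangeGameState stores it, prints its name for debugging and broadcasts it through an event dispatcher.
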(event `self.ReceiveTick`
  (params (DeltaSeconds :type "Float (single-precision)"))
  (set `self.TotalDeltaSeconds` (+ DeltaSeconds (`self.TotalDeltaSeconds`))))

(fn `ChangeGameState`
  (params (GameState :type "/Game/HackAndSlash/GameMode/EN_GameState Enum" :default "NewEnumerator0"))
  (set `self.TotalDeltaSeconds` 0.0)
  (if (`|EnumInequality` (`self.GameState`) GameState)
    (bind _output_get (set `self.GameState` GameState))
    (`KismetSystemLibrary.PrintString` (`KismetStringLibrary.Concat_StrStr` "ChangeGameState : " (`|GetEnumeratorNameAsString` _output_get)) true true (struct :`G` 0.66 :`B` 1.0 :`A` 1.0) 30.0)
    (`self.NewEventDispatcher_ChangeGameState` _output_get)))

(fn `UserConstructionScript`)