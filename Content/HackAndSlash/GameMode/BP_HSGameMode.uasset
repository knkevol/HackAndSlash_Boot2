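; BP_HSGameMode is the hack-and-slash game mode that drives match phases through BP_HSGameState.
; On BeginPlay it binds to the game state's change dispatcher and sets Ready, then Tick switches to Play once the state's elapsed time passes a short delay.
; EventChangeGameState gives game-only input with a hidden cursor, except in End, where it pauses the game and enables UI input with a visible cursor.
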(event `self.ReceiveBeginPlay`
  (bind _asbp_hsgame_state (cast `/Game/HackAndSlash/GameMode/BP_HSGameState` (`GameplayStatics.GetGameState`)))
  (add `/Game/HackAndSlash/GameMode/BP_HSGameState.NewEventDispatcher_ChangeGameState` _asbp_hsgame_state (`|CreateDelegate` :!event `EventChangeGameState`))
  (`/Game/HackAndSlash/GameMode/BP_HSGameState.ChangeGameState` _asbp_hsgame_state "NewEnumerator1"))

(event `self.ReceiveTick`
  (params (DeltaSeconds :type "Float (single-precision)"))
  (bind _asbp_hsgame_state (cast `/Game/HackAndSlash/GameMode/BP_HSGameState` (`GameplayStatics.GetGameState`)))
  (switch `/Game/HackAndSlash/GameMode/EN_GameState` (`/Game/HackAndSlash/GameMode/BP_HSGameState.GameState` _asbp_hsgame_state)
    (:`NewEnumerator1`
      (`self.StateReady` (`/Game/HackAndSlash/GameMode/BP_HSGameState.TotalDeltaSeconds` _asbp_hsgame_state) _asbp_hsgame_state))))

(fn `EventChangeGameState`
  (params (GameState :type "/Game/HackAndSlash/GameMode/EN_GameState Enum" :default "NewEnumerator0"))
  (bind _returnvalue (`GameplayStatics.GetPlayerController` 0))
  (bind _returnvalue_2 (`GameplayStatics.GetPlayerController` 0))
  (switch `/Game/HackAndSlash/GameMode/EN_GameState` GameState
    (:`NewEnumerator0`
      (`WidgetBlueprintLibrary.SetInputMode_GameOnly` _returnvalue :!label _label)
      (set `PlayerController.bShowMouseCursor` false _returnvalue))
    (:`NewEnumerator1`
      (goto _label))
    (:`NewEnumerator2`
      (goto _label))
    (:`NewEnumerator3`
      (`GameplayStatics.SetGamePaused` true)
      (`WidgetBlueprintLibrary.SetInputMode_GameAndUIEx` _returnvalue_2 null)
      (set `PlayerController.bShowMouseCursor` true _returnvalue_2))))

(fn `StateReady`
  (params (TotalDeltaSeconds :type "Float (double-precision)") (GameState :type "/Game/HackAndSlash/GameMode/BP_HSGameState Object Reference"))
  (if (>= TotalDeltaSeconds 6.0)
    (`/Game/HackAndSlash/GameMode/BP_HSGameState.ChangeGameState` GameState "NewEnumerator2")))

(fn `UserConstructionScript`)