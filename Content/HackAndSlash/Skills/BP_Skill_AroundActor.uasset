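; Hack-and-slash skill actor that orbits a Sphere on a SpringArm around its Instigator and damages what it reaches.
; DoApplyDamage nudges the arm's rotation, snaps the actor to the Instigator's location, then applies radial damage at the Sphere, ignoring the Instigator.
; BeginPlay calls this once if the game state is Play.
; The repeating-timer node is unconnected, and nothing here repeats the step.
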(event `self.ReceiveBeginPlay`
  (`parent.ReceiveBeginPlay`)
  (bind _asbp_hsgame_state (cast `/Game/HackAndSlash/GameMode/BP_HSGameState` (`GameplayStatics.GetGameState`)))
  (switch `/Game/HackAndSlash/GameMode/EN_GameState` (`/Game/HackAndSlash/GameMode/BP_HSGameState.GameState` _asbp_hsgame_state)
    (:`NewEnumerator2`
      (`self.DoApplyDamage`))))

(fn `AttachToCharacter`
  (`self.K2_SetActorLocation` (`self.K2_GetActorLocation` (`self.Instigator`))))

(fn `DoApplyDamage`
  (bind _instigator (`self.Instigator`))
  (`self.MoveAround`)
  (`GameplayStatics.ApplyRadialDamage` 50.0 (`SceneComponent.K2_GetComponentLocation` (`self.Sphere`)) (`self.Radius`) null (`|MakeArray` _instigator :!type "Actor Object Reference") self (`Pawn.GetController` _instigator)))

(fn `MoveAround`
  (`SceneComponent.K2_AddRelativeRotation` (`self.SpringArm`) (struct :`Yaw` 2.0) false false)
  (`self.AttachToCharacter`))

(fn `UserConstructionScript`
  (`parent.UserConstructionScript`))