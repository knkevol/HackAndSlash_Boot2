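; BP_Skill_Homing is a hack-and-slash skill projectile that homes in on a nearby target and explodes on overlap.
; While the game state is Play, each tick sphere-traces for a target, smoothly turns the Arrow toward it, and moves it forward by Speed per frame, unscaled by delta time.
; Cone overlap applies radial damage that ignores the Instigator, spawns an explosion effect and destroys the actor.
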(event `self.ReceiveBeginPlay`
  (`parent.ReceiveBeginPlay`))

(event `self.ReceiveTick`
  (params (DeltaSeconds :type "Float (single-precision)"))
  (bind _asbp_hsgame_state (cast `/Game/HackAndSlash/GameMode/BP_HSGameState` (`GameplayStatics.GetGameState`)))
  (switch `/Game/HackAndSlash/GameMode/EN_GameState` (`/Game/HackAndSlash/GameMode/BP_HSGameState.GameState` _asbp_hsgame_state)
    (:`NewEnumerator2`
      (if (not (`self.IsActorBeingDestroyed`))
        (`self.FindTarget`)
        (`self.RotateToTarget` DeltaSeconds)
        (`self.MoveForward` DeltaSeconds)))))

(event `self.Cone.OnComponentBeginOverlap`
  (params (OverlappedComponent :type "PrimitiveComponent Object Reference") (OtherActor :type "Actor Object Reference") (OtherComp :type "PrimitiveComponent Object Reference") (OtherBodyIndex :type Integer) (bFromSweep :type Boolean) (SweepResult :type "HitResult Structure (by ref)"))
  (bind (_returnvalue_location _returnvalue_rotation) (`KismetMathLibrary.BreakTransform` (`SceneComponent.GetRelativeTransform` (`self.Arrow`))))
  ;[0.15 0.15 0.15 0.5 10] collision 변경하여 적용해야됨
  (`self.DoApplyDamage`)
  (`NiagaraFunctionLibrary.SpawnSystemAtLocation` "/Niagara/DefaultAssets/Templates/Systems/SimpleExplosion.SimpleExplosion" _returnvalue_location _returnvalue_rotation (2.0 2.0 2.0))
  (`self.K2_DestroyActor`))

(event `self.ReceiveDestroyed`)

(fn `DoApplyDamage`
  (bind _instigator (`self.Instigator`))
  (`KismetSystemLibrary.DrawDebugSphere` (`SceneComponent.K2_GetComponentLocation` (`self.Arrow`)) (`self.Radius`) 12 (struct :`R` 1.0 :`G` 0.358605 :`B` 0.380096 :`A` 1.0) 1.0 1.0)
  (`GameplayStatics.ApplyRadialDamage` 50.0 (`SceneComponent.K2_GetComponentLocation` (`self.Arrow`)) (`self.Radius`) null (`|MakeArray` _instigator :!type "Actor Object Reference") self (`Pawn.GetController` _instigator)))

(fn `FindTarget`
  (bind _returnvalue (`SceneComponent.K2_GetComponentLocation` (`self.Arrow`)))
  ;[0.15 0.15 0.15 0.5 10] 거리체크없이 가까운액터 찾아줌(Radius = 탐색거리)
  (bind (_outhit _returnvalue_2) (`KismetSystemLibrary.SphereTraceSingleForObjects` :`Start` _returnvalue :`End` _returnvalue :`Radius` 1000.0 :`ObjectTypes` (`|MakeArray` "ObjectTypeQuery7" :!type "EObjectTypeQuery Enum") :`DrawDebugType` "ForOneFrame"))
  (if _returnvalue_2
    ; Monster
    (set `self.Target` (`.HitActor` (`GameplayStatics.BreakHitResult` _outhit)))))

(fn `MoveForward`
  (params (DeltaSeconds :type "Float (double-precision)"))
  (`SceneComponent.K2_AddWorldOffset` (`self.Arrow`) (* (`SceneComponent.GetForwardVector` (`self.Arrow`)) (`self.Speed`)) false false))

(fn `RotateToTarget`
  (params (DeltaSeconds :type "Float (double-precision)"))
  (bind _arrow (`self.Arrow`))
  (bind (_returnvalue_x _returnvalue_y) (`KismetMathLibrary.BreakVector` (`SceneComponent.K2_GetComponentLocation` _arrow)))
  (bind _target (`self.Target`)
    (:`then`
      (bind (_returnvalue_x_2 _returnvalue_y_2) (`KismetMathLibrary.BreakVector` (`self.K2_GetActorLocation` _target)))
      (`SceneComponent.K2_SetWorldRotation` (`self.Arrow`) (`KismetMathLibrary.RInterpTo` (`SceneComponent.K2_GetComponentRotation` _arrow) (`KismetMathLibrary.FindLookAtRotation` (`KismetMathLibrary.MakeVector` _returnvalue_x _returnvalue_y) (`KismetMathLibrary.MakeVector` _returnvalue_x_2 _returnvalue_y_2)) (`local.DeltaSeconds`) 5.0) false false))
    (:`else`)))

(fn `UserConstructionScript`
  (`parent.UserConstructionScript`))