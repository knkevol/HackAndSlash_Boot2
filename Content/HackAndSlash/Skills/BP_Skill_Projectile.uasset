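; Skill projectile for the hack-and-slash game that deals repeated area damage as it flies.
; Tick moves the Sphere component along its forward vector at constant speed, without sweep.
; A looping timer started on BeginPlay calls DoApplyDamage, which applies radial damage around the Sphere, excludes the Instigator so the hero is unharmed, and draws a debug sphere.
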(event `self.ReceiveBeginPlay`
  (`parent.ReceiveBeginPlay`)
  (`KismetSystemLibrary.K2_SetTimer` null "DoApplyDamage" 0.1 true))

(event `self.ReceiveTick`
  (params (DeltaSeconds :type "Float (single-precision)"))
  (`SceneComponent.K2_AddWorldOffset` (`self.Sphere`) (* (* DeltaSeconds 1000.0) (`SceneComponent.GetForwardVector` (`self.Sphere`))) false false))

(fn `DoApplyDamage`
  (bind _instigator (`self.Instigator`))
  (`KismetSystemLibrary.DrawDebugSphere` (`SceneComponent.K2_GetComponentLocation` (`self.Sphere`)) (`self.Radius`) 12 (struct :`R` 1.0 :`G` 0.358605 :`B` 0.380096 :`A` 1.0) 1.0 1.0)
  (`GameplayStatics.ApplyRadialDamage` 500.0 (`SceneComponent.K2_GetComponentLocation` (`self.Sphere`)) (`self.Radius`) null (`|MakeArray` _instigator :!type "Actor Object Reference") self (`Pawn.GetController` _instigator)))

(fn `UserConstructionScript`
  (`parent.UserConstructionScript`))