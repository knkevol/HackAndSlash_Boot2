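; Coin pickup item for the HackAndSlash game that spins in place and credits the collecting player.
; Tick applies a fixed relative rotation to the static mesh each frame, so spin speed depends on frame rate.
; When a pawn overlaps the mesh and has a BP_HSPlayerState, the coin calls AddCoin on that player state, then destroys itself.
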(event `self.ReceiveTick`
  (params (DeltaSeconds :type "Float (single-precision)"))
  (`parent.ReceiveTick` DeltaSeconds)
  (`SceneComponent.K2_AddRelativeRotation` (`self.StaticMesh`) (struct :`Yaw` 2.0) false false))

(event `self.StaticMesh.OnComponentBeginOverlap`
  (params (OverlappedComponent :type "PrimitiveComponent Object Reference") (OtherActor :type "Actor Object Reference") (OtherComp :type "PrimitiveComponent Object Reference") (OtherBodyIndex :type Integer) (bFromSweep :type Boolean) (SweepResult :type "HitResult Structure (by ref)"))
  (bind _aspawn (cast `Pawn` OtherActor))
  (bind _asbp_hsplayer_state (cast `/Game/HackAndSlash/GameMode/BP_HSPlayerState` (`Pawn.PlayerState` _aspawn)))
  (`/Game/HackAndSlash/GameMode/BP_HSPlayerState.AddCoin` _asbp_hsplayer_state)
  (`self.K2_DestroyActor`))

(fn `UserConstructionScript`
  (`parent.UserConstructionScript`))